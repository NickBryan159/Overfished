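; BP_Shark is the shark enemy in Overfished that rams the player's boat.
; It rotates to a fixed yaw on BeginPlay, then reacts to capsule overlaps with BP_Boat.
; On contact it calls GetRammed on the boat and stops its AI controller's brain logic for the RamCooldown delay, then restarts it.
; A leftover debug print fires after the cooldown.
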(event OnComponentBeginOverlap(CapsuleComponent)
  (params (OverlappedComponent :type Primitive%20Component%20Object%20Reference) (OtherActor :type Actor%20Object%20Reference) (OtherComp :type Primitive%20Component%20Object%20Reference) (OtherBodyIndex :type Integer) (bFromSweep :type Boolean) (SweepResult :type Hit%20Result%20Structure%20%28by%20ref%29))
  (bind _self self)
  (bind _returnvalue (AI|GetAIController _self))
  (bind _braincomponent (Variables|/Script/AIModule.AIController|GetBrainComponent _returnvalue))
  (bind _asbp_boat (Utilities|Casting|CastToBP_Boat OtherActor))
  (Default|GetRammed _asbp_boat)
  (AI|Logic|StopLogic _braincomponent "")
  (Utilities|FlowControl|Delay (Variables|Default|GetRam%20Cooldown))
  (AI|Logic|StartLogic _braincomponent)
  (Development|PrintString "Hello"))

(event EventBeginPlay
  (Transformation|SetActorRotation "-90.000000,0.000000,0.000000"))

(event Collision|EventActorBeginOverlap
  (params (OtherActor :type Actor%20Object%20Reference)))

(event EventTick
  (params (DeltaSeconds :type Float%20%28single-precision%29)))

(fn ConstructionScript)