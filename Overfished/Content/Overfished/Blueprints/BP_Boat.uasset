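; Player boat pawn for a fishing game, steered and braked through floating pawn movement and turned to face its direction of travel.
; Catching a fish overlapping the hook stops the boat, then requires button mashing followed by stick circles, tracked by angle wrap and a half-turn checkpoint.
; Billboard prompts and controller rumble signal each stage, and success destroys the fish and fires a caught callback.
; Cancelling or being rammed by another boat frees the fish.
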(event OnComponentEndOverlap(FishingHookCollider)
  (params (OverlappedComponent :type Primitive%20Component%20Object%20Reference) (OtherActor :type Actor%20Object%20Reference) (OtherComp :type Primitive%20Component%20Object%20Reference) (OtherBodyIndex :type Integer))
  ;[0.15 0.15 0.15 0.5] Check Fishing Hook for Fish For Catch UI
  (if (not (Utilities|Array|IsValidIndex (Collision|GetOverlappingActors (Variables|Default|GetFishingHookCollider) "/Game/OVERFISHED/Blueprints/BP_Fish.BP_Fish_C" :!class /Script/Engine.PrimitiveComponent)))
    (Development|SetHiddeninGame (Variables|Default|GetBillboard) true false)))

(event OnComponentBeginOverlap(FishingHookCollider)
  (params (OverlappedComponent :type Primitive%20Component%20Object%20Reference) (OtherActor :type Actor%20Object%20Reference) (OtherComp :type Primitive%20Component%20Object%20Reference) (OtherBodyIndex :type Integer) (bFromSweep :type Boolean) (SweepResult :type Hit%20Result%20Structure%20%28by%20ref%29))
  ;[0.15 0.15 0.15 0.5] Check Fishing Hook for Fish For Catch UI
  (Variables|Default|GetCanMashFish
    (:then)
    (:else
      (Variables|Default|GetCanReelFish
        (:then)
        (:else
          (Utilities|Casting|CastToBP_Fish OtherActor)
          (Rendering|Components|Sprite|SetSprite (Variables|Default|GetBillboard) "/Game/OVERFISHED/Textures/startFish.startFish")
          (Development|SetHiddeninGame (Variables|Default|GetBillboard) false false))))))

(event OnComponentHit(Box)
  (params (HitComponent :type Primitive%20Component%20Object%20Reference) (OtherActor :type Actor%20Object%20Reference) (OtherComp :type Primitive%20Component%20Object%20Reference) (NormalImpulse :type Vector :default "0, 0, 0") (Hit :type Hit%20Result%20Structure%20%28by%20ref%29))
  ;[0.15 0.15 0.15 0.5] Boat Crash
  (bind _asbp_boat (Utilities|Casting|CastToBP_Boat OtherActor))
  (CallFunction|GetRammed _asbp_boat)
  (Development|PrintString (Utilities|String|Append "HIT " (Utilities|GetDisplayName OtherActor)) true true "(R=1.000000,G=0.000000,B=0.333862,A=1.000000)"))

(event Custom|Set%20Boat%20Material
  ;[0.15 0.15 0.15 0.5] Set Boat Material
  (Rendering|Material|SetMaterial (Variables|Default|GetBoatUnderbelly) 0 (Variables|Default|GetPlayerMaterial)))

(event Custom|GetRammed
  (bind _currentselectedfish (Variables|Default|GetCurrentSelectedFish))
  (bind _floatingpawnmovement (Variables|Default|GetFloatingPawnMovement))
  ;[0.15 0.15 0.15 0.5] Unlobotomize fish when cancelled, reset mashing and reeling states
  (Variables|Default|GetCanMashFish
    (:then
      (Variables|Default|SetCanMashFish false))
    (:else
      _))
  (Variables|Default|GetCanReelFish
    (:then
      (Variables|Default|SetCanReelFish false))
    (:else
      _))
  (Utilities|IsValid _currentselectedfish
    (:Is%20Valid
      (Default|Freed _currentselectedfish) ; unlobotomize
      (Variables|/Script/Engine.FloatingPawnMovement|SetMaxSpeed _floatingpawnmovement 1.2e+03)
      (Variables|/Script/Engine.FloatingPawnMovement|SetDeceleration _floatingpawnmovement 1e+03)
      (Variables|Default|SetMashCounter 0.0)
      (Variables|Default|SetLastDegrees 0.0)
      (Variables|Default|SetTimesReeled 0))))

(event Custom|FinalizeCatch
  (bind _floatingpawnmovement (Variables|Default|GetFloatingPawnMovement))
  ;[0.15 0.15 0.15 0.5] Finish Fish Catching
  (Utilities|IsValid (Variables|Default|GetCurrentSelectedFish)
    (:Is%20Valid
      (Actor|DestroyActor (Variables|Default|GetCurrentSelectedFish))
      (Variables|Default|SetCurrentSelectedFish 0) ; Clear selelcted fish
      (Default|CallPlayerCaughtAFish(FishMurder))
      (Variables|/Script/Engine.FloatingPawnMovement|SetMaxSpeed _floatingpawnmovement 1.2e+03)
      (Variables|/Script/Engine.FloatingPawnMovement|SetDeceleration _floatingpawnmovement 1e+03)
      (Variables|Default|SetCanReelFish false)
      (Variables|Default|SetCanMashFish false)
      (Utilities|FlowControl|Delay 0.1)
      ;[0.15 0.15 0.15 0.5] play victory cha ching vibration
      (bind _asbp_boat_player_controller (Utilities|Casting|CastToBP_BoatPlayerController (Pawn|GetController))
        (:then
          (Game|Feedback|PlayDynamicForceFeedback _asbp_boat_player_controller 0.4 0.3 true false true false)
          (Game|Feedback|PlayDynamicForceFeedback _asbp_boat_player_controller 1.0 0.3 true true true true))
        (:CastFailed
          (Development|PrintString "FAILEDCAST"))))))

(event Custom|ResetDay
  ;[0.15 0.15 0.15 0.5] NEW DAY
  (Transformation|SetWorldLocation (Variables|Default|GetBox) (Variables|Default|GetStarting%20Location) false true))

(event Input|EnhancedActionEvents|EnhancedInputActionIA_Move
  (params (ActionValue :type Vector%202D%20Structure) (ElapsedSeconds :type Float%20%28double-precision%29) (TriggeredSeconds :type Float%20%28double-precision%29) (InputAction :type Input%20Action%20Object%20Reference :default "/Game/OVERFISHED/Input/IA_Move.IA_Move"))
  ;[0.15 0.15 0.15 0.5] Move
  (Variables|Default|GetIsBraking?
    (:then)
    (:else
      (Pawn|Input|AddMovementInput (Math|Vector|MakeVector (.x ActionValue) (.y ActionValue) 0.0) 1.0 false))))

(event Input|EnhancedActionEvents|EnhancedInputActionIA_Brake
  (params (ActionValue :type Boolean) (ElapsedSeconds :type Float%20%28double-precision%29) (TriggeredSeconds :type Float%20%28double-precision%29) (InputAction :type Input%20Action%20Object%20Reference :default "/Game/OVERFISHED/Input/IA_Brake.IA_Brake"))
  (bind _floatingpawnmovement (Variables|Default|GetFloatingPawnMovement))
  ;[0.15 0.15 0.15 0.5] Boat slow
  (:Triggered
    (Variables|Default|SetIsBraking? ActionValue)
    (Variables|/Script/Engine.FloatingPawnMovement|SetDeceleration _floatingpawnmovement 4e+03))
  (:Canceled
    (Variables|Default|SetIsBraking? ActionValue :!label _label)
    (Variables|/Script/Engine.FloatingPawnMovement|SetDeceleration _floatingpawnmovement 1e+03))
  (:Completed
    (goto _label)))

(event Input|EnhancedActionEvents|EnhancedInputActionIA_CatchFish
  (params (ActionValue :type Boolean) (ElapsedSeconds :type Float%20%28double-precision%29) (TriggeredSeconds :type Float%20%28double-precision%29) (InputAction :type Input%20Action%20Object%20Reference :default "/Game/OVERFISHED/Input/IA_CatchFish.IA_CatchFish"))
  (bind _floatingpawnmovement (Variables|Default|GetFloatingPawnMovement))
  ;[0.15 0.15 0.15 0.5] Catch Fish
  (:Started
    (Variables|Default|GetCanMashFish
      (:then)
      (:else
        (Variables|Default|GetCanReelFish
          (:then)
          (:else
            (bind _asbp_fish (Utilities|Casting|CastToBP_Fish (Utilities|Array|Get(acopy) (Collision|GetOverlappingActors (Variables|Default|GetFishingHookCollider) "/Game/OVERFISHED/Blueprints/BP_Fish.BP_Fish_C" :!class /Script/Engine.PrimitiveComponent))))
            (bind _output_get (Variables|Default|SetCurrentSelectedFish _asbp_fish))
            (Default|Caught _output_get) ; Lobotomize
            (Rendering|Components|Sprite|SetSprite (Variables|Default|GetBillboard) "/Game/OVERFISHED/Textures/mashFish.mashFish")
            (Variables|Default|SetCanMashFish true)
            (Variables|/Script/Engine.FloatingPawnMovement|SetMaxSpeed _floatingpawnmovement 0.0)
            (Variables|/Script/Engine.FloatingPawnMovement|SetDeceleration _floatingpawnmovement 999999.0)
            (Variables|Default|SetMashCounter 0.0)
            (bind _asbp_boat_player_controller (Utilities|Casting|CastToBP_BoatPlayerController (Pawn|GetController))
              (:then
                (Game|Feedback|PlayDynamicForceFeedback _asbp_boat_player_controller 0.75 0.2 true true true true))
              (:CastFailed
                (Development|PrintString "FAILEDCAST")))))))))

(event Input|EnhancedActionEvents|EnhancedInputActionIA_Mash
  (params (ActionValue :type Boolean) (ElapsedSeconds :type Float%20%28double-precision%29) (TriggeredSeconds :type Float%20%28double-precision%29) (InputAction :type Input%20Action%20Object%20Reference :default "/Game/OVERFISHED/Input/IA_Mash.IA_Mash"))
  ;[0.15 0.15 0.15 0.5] Mashing
  (:Started
    (Variables|Default|GetCanMashFish
      (:then
        (if (>= (Variables|Default|GetMashCounter) 9.0)
          (Variables|Default|SetMashCounter 0.0)
          (Variables|Default|SetTimesReeled 0)
          (Variables|Default|SetCanReelFish true)
          (Variables|Default|SetCanMashFish false)
          (Rendering|Components|Sprite|SetSprite (Variables|Default|GetBillboard) "/Game/OVERFISHED/Textures/rotatePrompt.rotatePrompt")
          ;[0.15 0.15 0.15 0.5] play rotate vibration as soon as you start
          (bind _asbp_boat_player_controller (Utilities|Casting|CastToBP_BoatPlayerController (Pawn|GetController))
            (:then
              (Game|Feedback|PlayDynamicForceFeedback _asbp_boat_player_controller 0.6 0.75 true false true false))
            (:CastFailed
              (Development|PrintString "FAILEDCAST")))
          (else
            ;;[0.15 0.15 0.15 0.5] On a Mash
            (bind _result (Math|Float|IncrementFloat (Variables|Default|GetMashCounter))
              (:%20%20
                (Development|PrintString (Utilities|String|ToString(Float) _result))
                (bind _asbp_boat_player_controller_2 (Utilities|Casting|CastToBP_BoatPlayerController (Pawn|GetController))
                  (:then
                    (Game|Feedback|PlayDynamicForceFeedback _asbp_boat_player_controller_2 0.25 0.2 false false false true))
                  (:CastFailed
                    (Development|PrintString "FAILEDCAST" true true "(R=1.000000,G=0.000000,B=0.000000,A=1.000000)"))))))))
      (:else))))

(event Input|EnhancedActionEvents|EnhancedInputActionIA_ReelCircle
  (params (ActionValue :type Vector%202D%20Structure) (ElapsedSeconds :type Float%20%28double-precision%29) (TriggeredSeconds :type Float%20%28double-precision%29) (InputAction :type Input%20Action%20Object%20Reference :default "/Game/OVERFISHED/Input/IA_ReelCircle.IA_ReelCircle"))
  ;[0.15 0.15 0.15 0.5] Reeling Logic and Behavior
  (if (Variables|Default|GetCanReelFish) ; Are we in the reeling stage of fishing?
    (Variables|Default|SetCurrentDegrees (+ (Class|KismetMathLibrary|DegAtan2 (.x ActionValue) (.y ActionValue)) 1.8e+02)) ; Current Angle in Degrees
    (Variables|Default|GetHit180? ; Have we hit 180 checkpoint on this cycle?\nIf we HAVENT -> Go check to see if we are at checkpoint\nIf we HAVE -> Great! Keep on with the checks.
      (:then
        _)
      (:else
        (Variables|Default|SetHit180? (Math|Float|InRange(Float) (Variables|Default|GetCurrentDegrees) 1.6e+02 2e+02))))
    (Variables|Default|SetDegreeDifferenceFromCurrentAndLast (- (Variables|Default|GetLastDegrees) (Variables|Default|GetCurrentDegrees))) ; Difference between Last and New Degree
    (if (not (< -3e+02 (Variables|Default|GetDegreeDifferenceFromCurrentAndLast))) ; Detect if degree chang is >300
      (Variables|Default|GetHit180? ; Check did we hit the 180 degree checkpoint?
        (:then
          (Math|Integer|IncrementInt (Variables|Default|GetTimesReeled) ; Increase Num Times Reeled
            (:%20%20
              (Variables|Default|SetHit180? false) ; Reset Checkpoint
              (Utilities|FlowControl|Sequence
                (:then_0
                  (if (< (Variables|Default|GetTimesReeled) 5)
                    ;[0.15 0.15 0.15 0.5] play vibration every time you complete a circuit, long but soft
                    (bind _asbp_boat_player_controller (Utilities|Casting|CastToBP_BoatPlayerController (Pawn|GetController))
                      (:then
                        (Game|Feedback|PlayDynamicForceFeedback _asbp_boat_player_controller 0.6 0.5 true false true false))
                      (:CastFailed
                        (Development|PrintString "FAILEDCAST")))))
                (:then_1
                  (Development|PrintText (Utilities|Text|FormatText "Current Degree: {deg} 
Difference between c&l degrees: {ldeg} 
CANSCORE {score} 
Hit180? {180} 
Times Reeled {TR}" (Variables|Default|GetCurrentDegrees) (Variables|Default|GetDegreeDifferenceFromCurrentAndLast) (Variables|Default|GetcanScorePoint) (Variables|Default|GetHit180?) (Variables|Default|GetTimesReeled)) true true "(R=0.119860,G=1.000000,B=0.836311,A=1.000000)" 0.05 :!label _label)
                  (Variables|Default|SetLastDegrees (Variables|Default|GetCurrentDegrees))
                  ;[0.15 0.15 0.15 0.5] If 10 reels, catch
                  (if (>= (Variables|Default|GetTimesReeled) 5)
                    (CallFunction|FinalizeCatch)
                    (Variables|Default|SetCanReelFish false)))))))
        (:else
          (Development|PrintString "No Score did not hit 180" true true "(R=1.000000,G=0.443527,B=0.000000,A=1.000000)")
          (goto _label)))
      (elif (> (Variables|Default|GetDegreeDifferenceFromCurrentAndLast) 0.0)
        (Variables|Default|SetcanScorePoint true) ; We are now allowed to score
        (goto _label)
        (else
          (Variables|Default|SetcanScorePoint false) ; Reeled backwards, can't score anymore
          (Development|PrintString "RESET" true true "(R=1.000000,G=0.000000,B=0.003964,A=1.000000)")
          (goto _label))))))

(event Input|EnhancedActionEvents|EnhancedInputActionIA_Cancel
  (params (ActionValue :type Boolean) (ElapsedSeconds :type Float%20%28double-precision%29) (TriggeredSeconds :type Float%20%28double-precision%29) (InputAction :type Input%20Action%20Object%20Reference :default "/Game/OVERFISHED/Input/IA_Cancel.IA_Cancel"))
  (bind _currentselectedfish (Variables|Default|GetCurrentSelectedFish))
  (bind _floatingpawnmovement (Variables|Default|GetFloatingPawnMovement))
  ;[0.15 0.15 0.15 0.5] Unlobotomize fish when cancelled, reset mashing and reeling states
  (Variables|Default|GetCanMashFish
    (:then
      (Variables|Default|SetCanMashFish false))
    (:else
      _))
  (Variables|Default|GetCanReelFish
    (:then
      (Variables|Default|SetCanReelFish false))
    (:else
      _))
  (Utilities|IsValid _currentselectedfish
    (:Is%20Valid
      (Default|Freed _currentselectedfish) ; unlobotomize
      (Variables|/Script/Engine.FloatingPawnMovement|SetMaxSpeed _floatingpawnmovement 1.2e+03)
      (Variables|/Script/Engine.FloatingPawnMovement|SetDeceleration _floatingpawnmovement 1e+03)
      (Variables|Default|SetMashCounter 0.0)
      (Variables|Default|SetLastDegrees 0.0)
      (Variables|Default|SetTimesReeled 0))))

(event EventBeginPlay
  ;[0.15 0.15 0.15 0.5] Begin Play
  (Variables|Default|SetStarting%20Location (Transformation|GetWorldLocation (Variables|Default|GetBox))))

(event EventTick
  (params (DeltaSeconds :type Float%20%28single-precision%29))
  ;[0.15 0.15 0.15 0.5] Tick
  (Transformation|SetWorldRotation (Variables|Default|GetBoatBase) (Math|Interpolation|RInterpTo (Transformation|GetWorldRotation (Variables|Default|GetBoatBase)) (Math|Rotator|MakeRotator (.roll (Math|Rotator|MakeRotfromX (Math|Vector|GetUnitDirection(Vector) (Variables|Default|GetLastPosition) (Transformation|GetActorLocation)))) 0.0 (.yaw (Math|Rotator|MakeRotfromX (Math|Vector|GetUnitDirection(Vector) (Variables|Default|GetLastPosition) (Transformation|GetActorLocation))))) (* (Math|Vector|VectorLength (Math|Vector|GetUnitDirection(Vector) (Variables|Default|GetLastPosition) (Transformation|GetActorLocation))) (Utilities|Time|GetWorldDeltaSeconds)) 1e+02) false false)
  (Variables|Default|SetLastPosition (Transformation|GetActorLocation)))

(fn ConstructionScript)