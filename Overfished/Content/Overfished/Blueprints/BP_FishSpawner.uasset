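; BP_FishSpawner populates an area of the level with BP_Fish actors.
; It spawns a configured number of fish on BeginPlay and again on OnReset, each at a random navigable point within SpawnRadius of the spawner.
; Each successfully spawned fish gets a type rolled from the spawner's per-type percentage weights, applied through SetQualityColor.
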(event Custom|SpawnFish
  (bind _randomlocation (Class|NavigationSystemV1|GetRandomLocationinNavigableRadius (Transformation|GetActorLocation) (Variables|Default|GetSpawn%20Radius) 0 0))
  (bind _returnvalue (Game|SpawnActorfromClass "/Game/Overfished/Blueprints/BP_Fish.BP_Fish_C" (Math|Conversions|ToTransform(Vector) _randomlocation) "AdjustIfPossibleButDontSpawnIfColliding" "MultiplyWithRoot" 0 0))
  (Utilities|IsValid _returnvalue
    (:Is%20Valid
      (bind _returnvalue_2 (Class|GetRandTypebyPercentLibrary|GetRandTypebyPercent (Variables|Default|GetBottomFeeder%25) (Variables|Default|GetSilverFish%25) (Variables|Default|GetGreenFish%25) (Variables|Default|GetShadowFish%25)))
      (Default|SetQualityColor _returnvalue _returnvalue_2))))

(event EventOnReset
  (for _index (range 0 (Variables|Default|GetNumberOfFish))
    (CallFunction|SpawnFish)))

(event EventBeginPlay
  (for _index (range 0 (Variables|Default|GetNumberOfFish))
    (CallFunction|SpawnFish)))

(fn ConstructionScript)